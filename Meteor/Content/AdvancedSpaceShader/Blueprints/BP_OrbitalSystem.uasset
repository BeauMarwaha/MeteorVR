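; BP_OrbitalSystem is an orbital system actor that makes attached BP_CelestialBody actors circle its center.
; Setup, run at construction and BeginPlay, gives each body a scene-component pivot aimed at it and parents the body to that pivot.
; Tick yaws each pivot at a rate falling with the square of the body's distance, tuned by BaseOrbitSpeed and DecayByDistance.
; ShowOrbits adds distance-scaled orbit meshes with dynamic materials.
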(event `self.ReceiveBeginPlay`
  (`self.Setup`))

(event `self.ReceiveTick`
  (params (DeltaSeconds :type "Float (single-precision)"))
  (bind _decay_by_distance (`self.Decay by distance`))
  (for (_array_element _array_index) (`self.Orbits`)
    (`SceneComponent.K2_AddLocalRotation` _array_element (`KismetMathLibrary.MakeRotator` 0.0 0.0 (/ (* DeltaSeconds (* (* (`self.Base orbit speed`) 1000000.0) _decay_by_distance)) (* (`KismetMathLibrary.VSizeSquared` (- (`self.K2_GetActorLocation`) (`self.K2_GetActorLocation` (`KismetArrayLibrary.Array_Get` (`self.Planets`) _array_index)))) (`KismetMathLibrary.MultiplyMultiply_FloatFloat` _decay_by_distance 2.0)))) false false)))

(fn `Setup`
  (`|ExecutionSequence`
    (:`then_0`
      (for _array_element (`self.GetAttachedActors`)
        (bind _asbp_celestial_body (cast `/Game/AdvancedSpaceShader/Blueprints/Utility/BP_CelestialBody` _array_element))
        (`KismetArrayLibrary.Array_AddUnique` (`self.Planets`) _asbp_celestial_body)))
    (:`then_1`
      (for _array_element_2 (`self.Planets`)
        (bind _returnvalue (`AddComponent|NODE_AddSceneComponent-2`))
        (`KismetArrayLibrary.Array_AddUnique` (`self.Orbits`) _returnvalue)
        (`SceneComponent.K2_SetRelativeRotation` _returnvalue (`KismetMathLibrary.FindLookAtRotation` (`SceneComponent.K2_GetComponentLocation` _returnvalue) (`self.K2_GetActorLocation` _array_element_2)) false false)
        (`self.K2_AttachToComponent` _array_element_2 _returnvalue "None" "KeepWorld" "KeepWorld" "KeepWorld" true)))
    (:`then_2`
      (if (`self.Show orbits`)
        (for (_array_element_3 _array_index) (`self.Orbits`)
          (bind _returnvalue_2 (`AddComponent|NODE_AddStaticMeshComponent-1`))
          (`SceneComponent.K2_AttachToComponent` _returnvalue_2 _array_element_3 "None" "KeepRelative" "KeepRelative" "KeepRelative" true)
          (bind _returnvalue_3 (`PrimitiveComponent.CreateDynamicMaterialInstance` _returnvalue_2 0 "/Game/AdvancedSpaceShader/Materials/Presets/Orbit.Orbit"))
          (`SceneComponent.SetRelativeScale3D` _returnvalue_2 (`KismetMathLibrary.Conv_DoubleToVector` (/ (`KismetMathLibrary.VSize` (- (`SceneComponent.K2_GetComponentLocation` _array_element_3) (`self.K2_GetActorLocation` (`KismetArrayLibrary.Array_Get` (`self.Planets`) _array_index)))) 100.0))))))))

(fn `UserConstructionScript`
  (`self.Setup`))