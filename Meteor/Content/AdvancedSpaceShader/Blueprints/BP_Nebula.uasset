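; Nebula actor that renders a space sphere through a dynamic material instance and supports fading its opacity.
; Construction creates the instance and seeds its CameraPosition parameter from the world origin location, scaled down there but refreshed at a divisor of one on Tick.
; Each Tick also eases Opacity toward OpacityTarget, and destroys the actor once it is nearly transparent and flagged Destroying.
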(event `self.ReceiveTick`
  (params (DeltaSeconds :type "Float (single-precision)"))
  (`self.UpdateMaterials`))

(fn `SafeDestroyActorComponent`
  (params (ActorComponent :type "ActorComponent Object Reference"))
  (if (!= ActorComponent null)
    (`ActorComponent.K2_DestroyComponent` ActorComponent)))

(fn `SetUpMaterials`
  (`MaterialInstanceDynamic.SetVectorParameterValue` (`self.SpaceSphereMaterial`) "CameraPosition" (`KismetMathLibrary.Conv_VectorToLinearColor` (/ (`KismetMathLibrary.Conv_IntVectorToVector` (`GameplayStatics.GetWorldOriginLocation`)) 1000.0))))

(fn `UpdateMaterials`
  (`|ExecutionSequence`
    (:`then_0`
      (`MaterialInstanceDynamic.SetVectorParameterValue` (`self.SpaceSphereMaterial`) "CameraPosition" (`KismetMathLibrary.Conv_VectorToLinearColor` (/ (`KismetMathLibrary.Conv_IntVectorToVector` (`GameplayStatics.GetWorldOriginLocation`)) 1.0))))
    (:`then_1`
      (bind _output_get (set `self.Opacity` (`KismetMathLibrary.FInterpTo` (`self.Opacity`) (`self.OpacityTarget`) (`GameplayStatics.GetWorldDeltaSeconds`) 0.5)))
      (`MaterialInstanceDynamic.SetScalarParameterValue` (`self.SpaceSphereMaterial`) "Opacity" _output_get)
      (if (and (<= _output_get 0.05) (`self.Destroying`))
        (`self.K2_DestroyActor`)))))

(fn `UserConstructionScript`
  (bind _spacesphere (`self.SpaceSphere`))
  (`|ExecutionSequence`
    (:`then_0`
      (bind _returnvalue (`PrimitiveComponent.CreateDynamicMaterialInstance` _spacesphere 0 (`PrimitiveComponent.GetMaterial` _spacesphere 0)))
      (set `self.SpaceSphereMaterial` _returnvalue))
    (:`then_3`
      (set `self.RandomStream` (`KismetMathLibrary.MakeRandomStream` 0)))
    (:`then_4`
      (`self.SetUpMaterials`))))