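; BP_Starfield is a starfield particle actor that fades its opacity and removes itself when nearly invisible.
; On BeginPlay it creates a dynamic material instance from the particle system's first material.
; Each tick it interpolates Opacity toward OpacityTarget, which this graph never sets, and writes it to the material's Opacity parameter.
; The actor destroys itself once Opacity falls to the low threshold.
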(event `self.ReceiveBeginPlay`
  (bind _returnvalue (`PrimitiveComponent.CreateDynamicMaterialInstance` (`self.ParticleSystem`) 0 (`PrimitiveComponent.GetMaterial` (`self.ParticleSystem`) 0)))
  (set `self.Material` _returnvalue))

(event `self.ReceiveTick`
  (params (DeltaSeconds :type "Float (single-precision)"))
  (bind _output_get (set `self.Opacity` (`KismetMathLibrary.FInterpTo` (`self.Opacity`) (`self.OpacityTarget`) DeltaSeconds 1.0)))
  (`MaterialInstanceDynamic.SetScalarParameterValue` (`self.Material`) "Opacity" _output_get)
  (if (<= _output_get 0.1)
    (`self.K2_DestroyActor`)))

(fn `UserConstructionScript`)