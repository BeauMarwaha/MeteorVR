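; BP_Universe builds the space backdrop around the player and shifts the world origin every tick to allow a near-infinite universe.
; On BeginPlay it spawns a starfield and a gas-cloud nebula, both attached to the player pawn.
; Each tick it also updates MegaGrid from the origin and pushes universe and nebula settings into each nebula's space-sphere material.
; CreateNebula can fade out an older nebula, but its re-creation call in Tick is disconnected.
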(event `self.ReceiveBeginPlay`
  (`self.CreateStarfield`)
  (`self.CreateNebula`))

(event `self.ReceiveTick`
  (params (DeltaSeconds :type "Float (single-precision)"))
  (bind _returnvalue (/ (`KismetMathLibrary.Conv_IntVectorToVector` (`GameplayStatics.GetWorldOriginLocation`)) (`self.Nebula Spatial Frequency`)))
  (`|ExecutionSequence`
    (:`then_0`
      ;[0.4118 0 1] Origin shifting to allow for a more or less infinite universe
      (`GameplayStatics.SetWorldOriginLocation` (`KismetMathLibrary.FTruncVector` (+ (`self.K2_GetActorLocation` (`GameplayStatics.GetPlayerPawn` 0)) (`KismetMathLibrary.Conv_IntVectorToVector` (`GameplayStatics.GetWorldOriginLocation`))))))
    (:`then_1`
      (if (not (`KismetMathLibrary.NearlyEqual_FloatFloat` (`KismetMathLibrary.VSize` _returnvalue) (`KismetMathLibrary.VSize` (`self.MegaGrid`)) 1.0))
        (set `self.MegaGrid` _returnvalue)))
    (:`then_2`
      (`self.UpdateMaterials`))))

(fn `CreateNebula`
  (bind _output (`|GetArrayItem` (`self.Nebulas`)))
  (`|ExecutionSequence`
    (:`then_0`
      (if (>= (`KismetArrayLibrary.Array_Length` (`self.Nebulas`)) 2)
        (set `/Game/AdvancedSpaceShader/Blueprints/BP_Nebula.OpacityTarget` 0.0 _output)
        (set `/Game/AdvancedSpaceShader/Blueprints/BP_Nebula.Destroying` true _output)
        (`KismetArrayLibrary.Array_Remove` (`self.Nebulas`))))
    (:`then_1`
      (bind _returnvalue (`|SpawnActorFromClass` "/Game/AdvancedSpaceShader/Blueprints/BP_Nebula.BP_Nebula_C" (`self.GetTransform` (`GameplayStatics.GetPlayerPawn` 0)) "AlwaysSpawn" "OverrideRootScale" null "/Game/AdvancedSpaceShader/Textures/GasClouds/GAS_Cloud1.GAS_Cloud1" 1.0 1.0 2.0 0.5 3.0 1 null))
      (`KismetArrayLibrary.Array_Add` (`self.Nebulas`) _returnvalue)
      (`self.K2_AttachToActor` _returnvalue (`GameplayStatics.GetPlayerPawn` 0) "None" "SnapToTarget" "SnapToTarget" "SnapToTarget" true))))

(fn `CreateStarfield`
  (bind _returnvalue (`|SpawnActorFromClass` "/Game/AdvancedSpaceShader/Blueprints/BP_Starfield.BP_Starfield_C" (`KismetMathLibrary.MakeTransform` (0.0 0.0 0.0)) "AlwaysSpawn" "OverrideRootScale" null null))
  (bind _output_get (set `self.Starfield` _returnvalue))
  (`self.K2_AttachToActor` _output_get (`GameplayStatics.GetPlayerPawn` 0) "None" "SnapToTarget" "SnapToTarget" "KeepWorld" true))

(fn `UpdateMaterials`
  (for _array_element (`self.Nebulas`)
    (`|ExecutionSequence`
      (:`then_0`
        (bind _spacespherematerial (`/Game/AdvancedSpaceShader/Blueprints/BP_Nebula.SpaceSphereMaterial` _array_element))
        (`MaterialInstanceDynamic.SetScalarParameterValue` _spacespherematerial "BackgroundRadiation" (`self.Background Radiation`)))
      (:`then_1`
        (`MaterialInstanceDynamic.SetScalarParameterValue` _spacespherematerial "NebulaBrightness" (`self.Nebula Brightness`)))
      (:`then_2`
        (`MaterialInstanceDynamic.SetScalarParameterValue` _spacespherematerial "NebulaSimplicity" (`self.Nebula Simplicity`)))
      (:`then_3`
        (`MaterialInstanceDynamic.SetScalarParameterValue` _spacespherematerial "NebulaCollapse" (`self.Nebula Collapse`)))
      (:`then_4`
        (`MaterialInstanceDynamic.SetVectorParameterValue` _spacespherematerial "OriginBackgroundRadiationColour" (`KismetMathLibrary.Conv_ColorToLinearColor` (`self.Origin Background Radiation Colour`))))
      (:`then_5`
        (`MaterialInstanceDynamic.SetScalarParameterValue` _spacespherematerial "UniverseScale" (`self.UniverseScale`)))
      (:`then_6`
        (`MaterialInstanceDynamic.SetScalarParameterValue` _spacespherematerial "OffsetRate" (`self.Nebula Spatial Frequency`))))))

(fn `UserConstructionScript`)