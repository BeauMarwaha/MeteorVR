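; BP_Sun is a configurable sun actor with a surface, optional solar flares and a point light.
; The construction script creates dynamic materials for both meshes, then UpdateMaterials pushes colour, brightness, sunspot and flare settings into them.
; The light follows inner colour and brightness, with source radius derived from actor scale.
; Disabling flares destroys that component, and each update ends by calling SunUpdated.
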(fn `SafeDestroyActorComponent`
  (params (`Actor component` :type "ActorComponent Object Reference"))
  (if (!= `Actor component` null)
    (`ActorComponent.K2_DestroyComponent` `Actor component`)))

(fn `UpdateMaterials`
  (bind _solarflarematerial (`self.SolarFlareMaterial`))
  (bind _pointlight (`self.PointLight`))
  (bind _sunmaterial (`self.SunMaterial`))
  (`|ExecutionSequence`
    (:`then_0`
      (`LightComponent.SetIntensity` _pointlight (* (`self.Brightness`) 2.0)))
    (:`then_1`
      (`LightComponent.SetLightColor` _pointlight (`self.Inner colour`) true))
    (:`then_2`
      (`PointLightComponent.SetAttenuationRadius` _pointlight (`self.Sun attenuation`)))
    (:`then_3`
      (`PointLightComponent.SetSourceRadius` _pointlight (`KismetMathLibrary.VSize` (`self.GetActorScale3D`))))
    (:`then_4`
      (`|ExecutionSequence`
        (:`then_0`
          (`MaterialInstanceDynamic.SetVectorParameterValue` _sunmaterial "Inner colour" (`self.Inner colour`)))
        (:`then_1`
          (`MaterialInstanceDynamic.SetVectorParameterValue` _sunmaterial "Outer colour" (`self.Outer colour`)))
        (:`then_2`
          (`MaterialInstanceDynamic.SetScalarParameterValue` _sunmaterial "Brightness" (`self.Brightness`)))
        (:`then_3`
          (`MaterialInstanceDynamic.SetScalarParameterValue` _sunmaterial "Fresnel power" (`self.Colour balance`)))
        (:`then_4`
          (`MaterialInstanceDynamic.SetScalarParameterValue` _sunmaterial "Sunspot strength" (`self.Sunspot strength`)))))
    (:`then_5`
      (if (`self.Solar flares`)
        (`|ExecutionSequence`
          (:`then_0`
            (`MaterialInstanceDynamic.SetVectorParameterValue` _solarflarematerial "Colour 1" (`self.Inner colour`)))
          (:`then_1`
            (`MaterialInstanceDynamic.SetVectorParameterValue` _solarflarematerial "Colour 2" (`self.Outer colour`)))
          (:`then_2`
            (`SceneComponent.SetRelativeScale3D` (`self.SolarFlare`) (`KismetMathLibrary.Conv_DoubleToVector` (`self.Solar flare scale`))))
          (:`then_3`
            (`MaterialInstanceDynamic.SetScalarParameterValue` _solarflarematerial "Brightness" (`self.Brightness`)))
          (:`then_4`
            (`MaterialInstanceDynamic.SetScalarParameterValue` _solarflarematerial "Opacity" (`self.Solar flare opacity`))))
        (else
          (`self.SafeDestroyActorComponent` (`self.SolarFlare`)))))
    (:`then_6`
      (`self.SunUpdated`))))

(fn `UserConstructionScript`
  (bind _solarflare (`self.SolarFlare`))
  (bind _sun (`self.Sun`))
  (`|ExecutionSequence`
    (:`then_0`
      (bind _returnvalue (`PrimitiveComponent.CreateDynamicMaterialInstance` _sun 0 (`PrimitiveComponent.GetMaterial` _sun 0)))
      (set `self.SunMaterial` _returnvalue))
    (:`then_1`
      (bind _returnvalue_2 (`PrimitiveComponent.CreateDynamicMaterialInstance` _solarflare 0 (`PrimitiveComponent.GetMaterial` _solarflare 0)))
      (set `self.SolarFlareMaterial` _returnvalue_2))
    (:`then_2`
      (`self.UpdateMaterials`))))