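; BP_RibCageBroken is a broken rib cage prop that a motion controller can pick up and drop.
; It adds an item icon on BeginPlay.
; Pickup, called by BP_MotionController, turns off mesh physics, attaches the root to the given component at its world transform, and stores the attach result in BeingHeld.
; Drop restores physics, detaches the actor and clears BeingHeld.
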(event `self.ReceiveBeginPlay`
  ;[1 1 1] Set Item Icon
  (`AddComponent|NODE_AddBP_ItemIcon-0`))

(event `/Game/VirtualRealityBP/Blueprints/PickupActorInterface.Pickup`
  (params (AttachTo :type "SceneComponent Object Reference"))
  ;[1 1 1] Pickup and Drop Actors
  (`PrimitiveComponent.SetSimulatePhysics` (`self.StaticMeshComponent`) false)
  (bind _returnvalue (`SceneComponent.K2_AttachToComponent` (`self.K2_GetRootComponent`) AttachTo "None" "KeepWorld" "KeepWorld" "KeepWorld" false))
  (set `self.BeingHeld` _returnvalue))

(event `/Game/VirtualRealityBP/Blueprints/PickupActorInterface.Drop`
  ;[1 1 1] Pickup and Drop Actors
  (`PrimitiveComponent.SetSimulatePhysics` (`self.StaticMeshComponent`) true)
  (`self.K2_DetachFromActor` "KeepWorld" "KeepWorld" "KeepWorld")
  (set `self.BeingHeld` false))

(fn `UserConstructionScript`)