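; BP_SpaceShipPart1 is a collectible spaceship piece picked up with a VR motion controller.
; Pickup clears the controller's attached actor instead of holding the piece, flags Part1Collected on the parent pawn, spawns a spark burst and destroys itself.
; BeginPlay adds an item icon.
; Tick pulses two point lights by lerping intensity up and down, flipping direction each second with a timer and boolean.
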(event `self.ReceiveBeginPlay`
  ;[1 1 1] Set Item Icon
  (`AddComponent|NODE_AddBP_ItemIcon-0`))

(event `/Game/VirtualRealityBP/Blueprints/PickupActorInterface.Pickup`
  (params (AttachTo :type "SceneComponent Object Reference"))
  ;[1 1 1] Collect Piece
  (bind _asmotion_controller_component (cast `MotionControllerComponent` AttachTo))
  (bind _asbp_motion_controller (cast `/Game/VirtualRealityBP/Blueprints/BP_MotionController` (`ActorComponent.GetOwner` _asmotion_controller_component)))
  (set `/Game/VirtualRealityBP/Blueprints/BP_MotionController.AttachedActor` null _asbp_motion_controller)
  (set `/Game/VirtualRealityBP/Blueprints/MotionControllerPawn.Part1Collected` true (`/Game/VirtualRealityBP/Blueprints/BP_MotionController.ParentPawn` _asbp_motion_controller))
  (`GameplayStatics.SpawnEmitterAtLocation` "/Game/Content/Particles/P_SparksOnce.P_SparksOnce" (`SceneComponent.K2_GetComponentLocation` (`self.StaticMeshComponent`)) (struct) (5.0 5.0 5.0))
  (`self.K2_DestroyActor`))

(event `self.ReceiveTick`
  (params (DeltaSeconds :type "Float (single-precision)"))
  (bind _lighttiming (`self.LightTiming`))
  (bind _returnvalue (`KismetMathLibrary.Lerp` 20.0 500.0 _lighttiming))
  (bind _returnvalue_2 (`KismetMathLibrary.Lerp` 500.0 20.0 _lighttiming))
  ;[1 1 1] Have Light Fade In And Out In Intenstity Over Time
  (set `self.LightTiming` (+ DeltaSeconds _lighttiming))
  (if (`self.ChangeType`)
    (if (>= _lighttiming 1.0)
      (set `self.LightTiming` 0.0)
      (set `self.ChangeType` false)
      (else
        (`LightComponent.SetIntensity` (`self.PointLight`) _returnvalue_2)
        (`LightComponent.SetIntensity` (`self.PointLight1`) _returnvalue_2)))
    (elif (>= _lighttiming 1.0)
      (set `self.LightTiming` 0.0)
      (set `self.ChangeType` true)
      (else
        (`LightComponent.SetIntensity` (`self.PointLight`) _returnvalue)
        (`LightComponent.SetIntensity` (`self.PointLight1`) _returnvalue)))))

(fn `UserConstructionScript`)