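; BP_IceBlock is an ice block that melts when a BP_Torch overlaps its trigger box, revealing a spaceship part inside.
; The overlap plays one-shot melt animations on the block and its puddle.
; After a fixed delay it destroys the InsideItem component and spawns BP_SpaceShipPart3 at the root transform with physics simulation disabled.
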(event `self.TriggerBox.OnComponentBeginOverlap`
  (params (OverlappedComponent :type "PrimitiveComponent Object Reference") (OtherActor :type "Actor Object Reference") (OtherComp :type "PrimitiveComponent Object Reference") (OtherBodyIndex :type Integer) (bFromSweep :type Boolean) (SweepResult :type "HitResult Structure (by ref)"))
  ;[1 1 1] Play Animations, Destroy The Ice Block, And Spawn The Inside Item When Interacted With The Torch
  (cast `/Game/Content/Blueprints/BP_Torch` OtherActor)
  (`SkeletalMeshComponent.PlayAnimation` (`self.IceBlock`) "/Game/Content/Animations/A_IceBlock_Melt.A_IceBlock_Melt" false)
  (`SkeletalMeshComponent.PlayAnimation` (`self.IcePuddle`) "/Game/Content/Animations/A_IcePuddle_Melt.A_IcePuddle_Melt" false)
  (`KismetSystemLibrary.Delay` 5.0)
  (`ActorComponent.K2_DestroyComponent` (`self.InsideItem`))
  (bind _returnvalue (`|SpawnActorFromClass` "/Game/Content/Blueprints/BP_SpaceShipPart3.BP_SpaceShipPart3_C" (`SceneComponent.K2_GetComponentToWorld` (`self.DefaultSceneRoot`)) "AlwaysSpawn" "OverrideRootScale" null null))
  (`PrimitiveComponent.SetSimulatePhysics` (`StaticMeshActor.StaticMeshComponent` _returnvalue) false))

(fn `UserConstructionScript`)