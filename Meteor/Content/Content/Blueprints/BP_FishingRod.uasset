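; BP_FishingRod is a fishing rod actor that BP_MotionController can pick up and drop, and it adds an item icon on BeginPlay.
; Pickup stops mesh physics, attaches the root to the supplied component, records the result in BeingHeld, then simulates only bones below JT_Base so they move physically while held.
; Drop restores physics on the whole skeletal mesh, detaches the actor and clears BeingHeld.
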(event `self.ReceiveBeginPlay`
  ;[1 1 1] Set Item Icon
  (`AddComponent|NODE_AddBP_ItemIcon-0`))

(event `/Game/VirtualRealityBP/Blueprints/PickupActorInterface.Pickup`
  (params (AttachTo :type "SceneComponent Object Reference"))
  ;[1 1 1] Pickup and Drop Skeletal Mesh Actors
  (`PrimitiveComponent.SetSimulatePhysics` (`self.SkeletalMeshComponent`) false)
  (bind _returnvalue (`SceneComponent.K2_AttachToComponent` (`self.K2_GetRootComponent`) AttachTo "None" "KeepWorld" "KeepWorld" "KeepWorld" false))
  (set `self.BeingHeld` _returnvalue)
  (`SkeletalMeshComponent.SetAllBodiesBelowSimulatePhysics` (`self.SkeletalMeshComponent`) "JT_Base" true false))

(event `/Game/VirtualRealityBP/Blueprints/PickupActorInterface.Drop`
  ;[1 1 1] Pickup and Drop Skeletal Mesh Actors
  (`SkeletalMeshComponent.SetAllBodiesBelowSimulatePhysics` (`self.SkeletalMeshComponent`) "JT_Base" true true)
  (`PrimitiveComponent.SetSimulatePhysics` (`self.SkeletalMeshComponent`) true)
  (`self.K2_DetachFromActor` "KeepWorld" "KeepWorld" "KeepWorld")
  (set `self.BeingHeld` false))

(fn `UserConstructionScript`)