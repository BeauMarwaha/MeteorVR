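; Fish actor that loops a swim animation while its Fish mesh travels along a spline path.
; Each Tick advances a distance along the spline, resetting to zero at the end so the route repeats.
; The mesh follows the spline's world location and rotation, with a downward offset and a half-turn in yaw.
; The distance step divides Speed by DeltaSeconds rather than multiplying, so movement speed varies with frame rate.
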(event `self.ReceiveBeginPlay`
  ;[1 1 1] Start Playing Swim Animation
  (`SkeletalMeshComponent.PlayAnimation` (`self.Fish`) "/Game/Content/Animations/A_Fish01_Swim.A_Fish01_Swim" true))

(event `self.ReceiveTick`
  (params (DeltaSeconds :type "Float (single-precision)"))
  (bind _currentdistancedownspline (`self.CurrentDistanceDownSpline`))
  (bind _spline (`self.Spline`))
  ;[1 1 1] Calculate New Current Distance Down Spline
  (set `self.CurrentDistanceDownSpline` (+ (/ (/ (`self.Speed`) 100.0) DeltaSeconds) (`self.CurrentDistanceDownSpline`)))
  ;[1 1 1] Reset Distance If It Exceeds Spline Length
  (if (>= (`self.CurrentDistanceDownSpline`) (`SplineComponent.GetSplineLength` (`self.Spline`)))
    (set `self.CurrentDistanceDownSpline` 0.0))
  ;[1 1 1] Move The Actor Along A Defined Spline Path
  (`SceneComponent.K2_SetWorldTransform` (`self.Fish`) (`KismetMathLibrary.MakeTransform` (`KismetMathLibrary.MakeVector` (.x (`SplineComponent.GetLocationAtDistanceAlongSpline` _spline _currentdistancedownspline "World")) (.y (`SplineComponent.GetLocationAtDistanceAlongSpline` _spline _currentdistancedownspline "World")) (- (.z (`SplineComponent.GetLocationAtDistanceAlongSpline` _spline _currentdistancedownspline "World")) 25.0)) (`KismetMathLibrary.MakeRotator` (.roll (`SplineComponent.GetRotationAtDistanceAlongSpline` _spline _currentdistancedownspline "World")) (.pitch (`SplineComponent.GetRotationAtDistanceAlongSpline` _spline _currentdistancedownspline "World")) (+ (.yaw (`SplineComponent.GetRotationAtDistanceAlongSpline` _spline _currentdistancedownspline "World")) 180.0))) false false))

(fn `UserConstructionScript`)