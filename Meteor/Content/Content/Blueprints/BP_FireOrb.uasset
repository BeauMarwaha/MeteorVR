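; BP_FireOrb is a VR pickup item that combines with a stick to make a torch.
; Pickup and Drop, called by the motion controller, toggle physics, attach or detach the orb and update its held-item info.
; On a hit, the BPItemCombination component receives BP_Stick as the class to combine and BP_Torch as the class to spawn.
; It also adds its item icon on BeginPlay.
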(event `self.ReceiveBeginPlay`
  ;[1 1 1] Set Item Icon
  (`AddComponent|NODE_AddBP_ItemIcon-0`))

(event `/Game/VirtualRealityBP/Blueprints/PickupActorInterface.Pickup`
  (params (AttachTo :type "SceneComponent Object Reference"))
  (bind _bp_helditeminfo (`self.BP_HeldItemInfo`))
  ;[1 1 1] Pickup and Drop Actors
  (`PrimitiveComponent.SetSimulatePhysics` (`self.StaticMeshComponent`) false)
  (bind _returnvalue (`SceneComponent.K2_AttachToComponent` (`self.K2_GetRootComponent`) AttachTo "None" "KeepWorld" "KeepWorld" "KeepWorld" false))
  (set `/Game/Content/Blueprints/ActorComponents/BP_HeldItemInfo.BeingHeld` _returnvalue _bp_helditeminfo)
  (set `/Game/Content/Blueprints/ActorComponents/BP_HeldItemInfo.HeldBy` AttachTo _bp_helditeminfo))

(event `/Game/VirtualRealityBP/Blueprints/PickupActorInterface.Drop`
  (bind _bp_helditeminfo (`self.BP_HeldItemInfo`))
  ;[1 1 1] Pickup and Drop Actors
  (`PrimitiveComponent.SetSimulatePhysics` (`self.StaticMeshComponent`) true)
  (`self.K2_DetachFromActor` "KeepWorld" "KeepWorld" "KeepWorld")
  (set `/Game/Content/Blueprints/ActorComponents/BP_HeldItemInfo.BeingHeld` false _bp_helditeminfo)
  (set `/Game/Content/Blueprints/ActorComponents/BP_HeldItemInfo.HeldBy` null _bp_helditeminfo))

(event `self.ReceiveHit`
  (params (MyComp :type "PrimitiveComponent Object Reference") (Other :type "Actor Object Reference") (OtherComp :type "PrimitiveComponent Object Reference") (bSelfMoved :type Boolean) (HitLocation :type "Vector Structure") (HitNormal :type "Vector Structure") (NormalImpulse :type "Vector Structure") (Hit :type "HitResult Structure (by ref)"))
  ;[1 1 1] Combining With Stick to Make Torch
  (`/Game/Content/Blueprints/ActorComponents/BP_ItemCombination.CombineItems` (`self.BP_ItemCombination`) self Other Hit "/Game/Content/Blueprints/BP_Stick.BP_Stick_C" "/Game/Content/Blueprints/BP_Torch.BP_Torch_C"))

(fn `UserConstructionScript`)