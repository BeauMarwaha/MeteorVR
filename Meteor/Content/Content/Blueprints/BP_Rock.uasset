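; BP_Rock is a physics rock that can be picked up, dropped and combined with a stick to craft an axe.
; BP_MotionController calls Pickup to disable physics and attach it, while Drop detaches it and restores physics.
; On hitting a BP_Stick while neither is held, it plays an explosion, destroys both actors and spawns BP_Axe at the impact point.
; It also adds an item icon on BeginPlay.
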(event `self.ReceiveBeginPlay`
  ;[1 1 1] Set Item Icon
  (`AddComponent|NODE_AddBP_ItemIcon-0`))

(event `/Game/VirtualRealityBP/Blueprints/PickupActorInterface.Pickup`
  (params (AttachTo :type "SceneComponent Object Reference"))
  ;[1 1 1] Pickup and Drop Actors
  (`PrimitiveComponent.SetSimulatePhysics` (`self.StaticMeshComponent`) false)
  (bind _returnvalue (`SceneComponent.K2_AttachToComponent` (`self.K2_GetRootComponent`) AttachTo "None" "KeepWorld" "KeepWorld" "KeepWorld" false))
  (set `self.BeingHeld` _returnvalue))

(event `/Game/VirtualRealityBP/Blueprints/PickupActorInterface.Drop`
  ;[1 1 1] Pickup and Drop Actors
  (`PrimitiveComponent.SetSimulatePhysics` (`self.StaticMeshComponent`) true)
  (`self.K2_DetachFromActor` "KeepWorld" "KeepWorld" "KeepWorld")
  (set `self.BeingHeld` false))

(event `self.ReceiveHit`
  (params (MyComp :type "PrimitiveComponent Object Reference") (Other :type "Actor Object Reference") (OtherComp :type "PrimitiveComponent Object Reference") (bSelfMoved :type Boolean) (HitLocation :type "Vector Structure") (HitNormal :type "Vector Structure") (NormalImpulse :type "Vector Structure") (Hit :type "HitResult Structure (by ref)"))
  (bind (_bblockinghit _binitialoverlap _time _distance _location _impactpoint) (`GameplayStatics.BreakHitResult` Hit))
  ;[1 1 1] Combining With Stick to Make Axe
  (if (not (`self.BeingHeld`))
    (bind _asbp_stick (cast `/Game/Content/Blueprints/BP_Stick` Other))
    (if (not (`/Game/Content/Blueprints/BP_Stick.BeingHeld` _asbp_stick))
      (`GameplayStatics.SpawnEmitterAtLocation` "/Game/StarterContent/Particles/P_Explosion.P_Explosion" _impactpoint (struct) (5.0 5.0 5.0))
      (`self.K2_DestroyActor` Other)
      (`self.K2_DestroyActor`)
      (`|SpawnActorFromClass` "/Game/Content/Blueprints/BP_Axe.BP_Axe_C" (`KismetMathLibrary.Conv_VectorToTransform` _impactpoint) "AlwaysSpawn" "OverrideRootScale" null null))))

(event `Key|MotionController_Left_Trigger`
  (params (Key :type "Key Structure"))
  ;[1 1 1] Combining With Stick to Make Axe
)

(fn `UserConstructionScript`)