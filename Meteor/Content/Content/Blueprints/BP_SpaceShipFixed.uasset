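; Spaceship actor that hovers in place and pulses eight point lights.
; BeginPlay starts two timelines that alternate endlessly, each setting the mesh's relative location to a lerp between the actor's world location and a small up or down Z offset.
; Tick accumulates a one-second timer and flips a boolean at each end to ramp all light intensities between dim and bright.
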(event `self.ReceiveBeginPlay`
  (bind _returnvalue (`self.K2_GetActorLocation`))
  (bind _returnvalue_2 (`self.K2_GetActorLocation`))
  ;[1 1 1] LERP Location Up And Down To Have Floating Effect
  (bind (_direction _newtrack_0) (`Timeline|Timeline_0` :!via `PlayFromStart` :!label _label)
    (:`Update`
      (`SceneComponent.K2_SetRelativeLocation` (`self.StaticMeshComponent`) (`KismetMathLibrary.VLerp` _returnvalue (+ _returnvalue (0.0 0.0 0.15)) _newtrack_0) false false))
    (:`Finished`
      (bind (_direction_2 _newtrack_0_2) (`Timeline|Timeline_1` :!via `PlayFromStart`)
        (:`Update`
          (`SceneComponent.K2_SetRelativeLocation` (`self.StaticMeshComponent`) (`KismetMathLibrary.VLerp` _returnvalue_2 (+ _returnvalue_2 (0.0 0.0 -0.15)) _newtrack_0_2) false false))
        (:`Finished`
          (goto _label :!via `PlayFromStart`))))))

(event `self.ReceiveTick`
  (params (DeltaSeconds :type "Float (single-precision)"))
  (bind _lighttiming (`self.LightTiming`))
  (bind _returnvalue (`KismetMathLibrary.Lerp` 20.0 300.0 _lighttiming))
  (bind _returnvalue_2 (`KismetMathLibrary.Lerp` 300.0 20.0 _lighttiming))
  ;[1 1 1] Have Light Fade In And Out In Intenstity Over Time
  (set `self.LightTiming` (+ DeltaSeconds _lighttiming))
  (if (`self.ChangeType`)
    (if (>= _lighttiming 1.0)
      (set `self.LightTiming` 0.0)
      (set `self.ChangeType` false)
      (else
        (`LightComponent.SetIntensity` (`self.PointLight`) _returnvalue_2)
        (`LightComponent.SetIntensity` (`self.PointLight1`) _returnvalue_2)
        (`LightComponent.SetIntensity` (`self.PointLight2`) _returnvalue_2)
        (`LightComponent.SetIntensity` (`self.PointLight3`) _returnvalue_2)
        (`LightComponent.SetIntensity` (`self.PointLight4`) _returnvalue_2)
        (`LightComponent.SetIntensity` (`self.PointLight5`) _returnvalue_2)
        (`LightComponent.SetIntensity` (`self.PointLight6`) _returnvalue_2)
        (`LightComponent.SetIntensity` (`self.PointLight7`) _returnvalue_2)))
    (elif (>= _lighttiming 1.0)
      (set `self.LightTiming` 0.0)
      (set `self.ChangeType` true)
      (else
        (`LightComponent.SetIntensity` (`self.PointLight`) _returnvalue)
        (`LightComponent.SetIntensity` (`self.PointLight1`) _returnvalue)
        (`LightComponent.SetIntensity` (`self.PointLight2`) _returnvalue)
        (`LightComponent.SetIntensity` (`self.PointLight3`) _returnvalue)
        (`LightComponent.SetIntensity` (`self.PointLight4`) _returnvalue)
        (`LightComponent.SetIntensity` (`self.PointLight5`) _returnvalue)
        (`LightComponent.SetIntensity` (`self.PointLight6`) _returnvalue)
        (`LightComponent.SetIntensity` (`self.PointLight7`) _returnvalue)))))

(fn `UserConstructionScript`)