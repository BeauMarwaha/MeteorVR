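; BP_MainTree is a choppable tree that breaks into a stump and a top when hit by a BP_Axe.
; On that hit it destroys itself, spawns BP_MainTreeStump at its transform and BP_MainTreeTop raised above it.
; The new top gets physics simulation and gravity enabled so it can fall.
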(event `self.ReceiveHit`
  (params (MyComp :type "PrimitiveComponent Object Reference") (Other :type "Actor Object Reference") (OtherComp :type "PrimitiveComponent Object Reference") (bSelfMoved :type Boolean) (HitLocation :type "Vector Structure") (HitNormal :type "Vector Structure") (NormalImpulse :type "Vector Structure") (Hit :type "HitResult Structure (by ref)"))
  (bind _returnvalue (`self.GetTransform`))
  ;[1 1 1] Pickup Actor should break off rib into hand and spawn broken ribs in its place
  (if (`KismetMathLibrary.ClassIsChildOf` (`GameplayStatics.GetObjectClass` Other) "/Game/Content/Blueprints/BP_Axe.BP_Axe_C")
    (`self.K2_DestroyActor`)
    (`|SpawnActorFromClass` "/Game/Content/Blueprints/BP_MainTreeStump.BP_MainTreeStump_C" _returnvalue "AlwaysSpawn" "OverrideRootScale" null null)
    (bind _returnvalue_2 (`|SpawnActorFromClass` "/Game/Content/Blueprints/BP_MainTreeTop.BP_MainTreeTop_C" (`KismetMathLibrary.MakeTransform` (+ (.location _returnvalue) (0.0 0.0 100.0)) (.rotation _returnvalue) (.scale _returnvalue)) "AlwaysSpawn" "OverrideRootScale" null null))
    (bind _staticmeshcomponent (`StaticMeshActor.StaticMeshComponent` _returnvalue_2))
    (`PrimitiveComponent.SetSimulatePhysics` _staticmeshcomponent true)
    (`PrimitiveComponent.SetEnableGravity` _staticmeshcomponent true)))

(fn `UserConstructionScript`)