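; BP_SpaceShipPart2 is the second collectible spaceship piece, picked up with a motion controller and consumed on grab.
; On BeginPlay it adds an item icon.
; When BP_MotionController calls Pickup, it clears that controller's AttachedActor instead of attaching, and sets Part2Collected on the controller's parent pawn.
; It then spawns a spark burst at its mesh and destroys itself.
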(event `self.ReceiveBeginPlay`
  ;[1 1 1] Set Item Icon
  (`AddComponent|NODE_AddBP_ItemIcon-0`))

(event `/Game/VirtualRealityBP/Blueprints/PickupActorInterface.Pickup`
  (params (AttachTo :type "SceneComponent Object Reference"))
  ;[1 1 1] Collect Piece
  (bind _asmotion_controller_component (cast `MotionControllerComponent` AttachTo))
  (bind _asbp_motion_controller (cast `/Game/VirtualRealityBP/Blueprints/BP_MotionController` (`ActorComponent.GetOwner` _asmotion_controller_component)))
  (set `/Game/VirtualRealityBP/Blueprints/BP_MotionController.AttachedActor` null _asbp_motion_controller)
  (set `/Game/VirtualRealityBP/Blueprints/MotionControllerPawn.Part2Collected` true (`/Game/VirtualRealityBP/Blueprints/BP_MotionController.ParentPawn` _asbp_motion_controller))
  (`GameplayStatics.SpawnEmitterAtLocation` "/Game/Content/Particles/P_SparksOnce.P_SparksOnce" (`SceneComponent.K2_GetComponentLocation` (`self.StaticMeshComponent`)) (struct) (5.0 5.0 5.0))
  (`self.K2_DestroyActor`))

(fn `UserConstructionScript`)