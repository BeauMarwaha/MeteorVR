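; BP_ItemCombination provides CombineItems, which merges two colliding VR items into a new actor when the hit object matches a given class.
; It reads each item's BP_HeldItemInfo, then plays an explosion and destroys both originals.
; If one item is held, the result spawns at that motion controller and becomes its held item; if neither, at the impact point.
; Combining two held items does nothing, as that branch is disconnected.
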(fn `CombineItems`
  (params (MainObject :type "Actor Object Reference") (HitObject :type "Actor Object Reference") (HitInfo :type "HitResult Structure") (ObjectClassToCombine :type "Actor Class Reference") (ObjectClassToSpawn :type "Actor Class Reference"))
  (bind (_bblockinghit _binitialoverlap _time _distance _location _impactpoint) (`GameplayStatics.BreakHitResult` HitInfo))
  (bind _returnvalue (`Actor.GetComponentByClass` HitObject "/Game/Content/Blueprints/BP_HeldItemInfo.BP_HeldItemInfo_C"))
  (bind _heldby (`/Game/Content/Blueprints/BP_HeldItemInfo.HeldBy` (`Actor.GetComponentByClass` MainObject "/Game/Content/Blueprints/BP_HeldItemInfo.BP_HeldItemInfo_C")))
  (bind _beingheld (`/Game/Content/Blueprints/BP_HeldItemInfo.BeingHeld` _returnvalue))
  (bind _heldby_2 (`/Game/Content/Blueprints/BP_HeldItemInfo.HeldBy` _returnvalue))
  ;[1 1 1] Check To Make Sure Colliding Object Is the Type We Want
  (if (`KismetMathLibrary.ClassIsChildOf` (`GameplayStatics.GetObjectClass` HitObject) ObjectClassToCombine)
    ;[1 1 1] Check If The Main Object Is Being Held
    (if (`/Game/Content/Blueprints/BP_HeldItemInfo.BeingHeld` (`Actor.GetComponentByClass` MainObject "/Game/Content/Blueprints/BP_HeldItemInfo.BP_HeldItemInfo_C"))
      ;[1 1 1] Check To See If The Colliding Object Is Being Held
      (if (not _beingheld)
        ;[1 1 1] Player Holding Main Object And Not Holding Colliding Object
        (bind _asbp_motion_controller (cast `/Game/VirtualRealityBP/Blueprints/BP_MotionController` (`self.GetOwner` _heldby)))
        (bind _motioncontroller (`/Game/VirtualRealityBP/Blueprints/BP_MotionController.MotionController` _asbp_motion_controller))
        (`GameplayStatics.SpawnEmitterAtLocation` "/Game/StarterContent/Particles/P_Explosion.P_Explosion" (`SceneComponent.K2_GetComponentLocation` _motioncontroller) (struct) (5.0 5.0 5.0))
        (bind _returnvalue_2 (`|SpawnActorFromClass` ObjectClassToSpawn (`SceneComponent.K2_GetComponentToWorld` _motioncontroller) "AlwaysSpawn" "OverrideRootScale" null null))
        (set `/Game/VirtualRealityBP/Blueprints/BP_MotionController.AttachedActor` _returnvalue_2 _asbp_motion_controller)
        (message `/Game/VirtualRealityBP/Blueprints/PickupActorInterface.Pickup` _returnvalue_2 _heldby)
        (`Actor.K2_DestroyActor` HitObject)
        (`Actor.K2_DestroyActor` MainObject))
      (elif _beingheld
        ;[1 1 1] Player Not Holding Main Object And Holding Colliding Object
        (bind _asbp_motion_controller_2 (cast `/Game/VirtualRealityBP/Blueprints/BP_MotionController` (`self.GetOwner` _heldby_2)))
        (bind _motioncontroller_2 (`/Game/VirtualRealityBP/Blueprints/BP_MotionController.MotionController` _asbp_motion_controller_2))
        (`GameplayStatics.SpawnEmitterAtLocation` "/Game/StarterContent/Particles/P_Explosion.P_Explosion" (`SceneComponent.K2_GetComponentLocation` _motioncontroller_2) (struct) (5.0 5.0 5.0))
        (bind _returnvalue_3 (`|SpawnActorFromClass` ObjectClassToSpawn (`SceneComponent.K2_GetComponentToWorld` _motioncontroller_2) "Undefined" "OverrideRootScale" null null))
        (set `/Game/VirtualRealityBP/Blueprints/BP_MotionController.AttachedActor` _returnvalue_3 _asbp_motion_controller_2)
        (message `/Game/VirtualRealityBP/Blueprints/PickupActorInterface.Pickup` _returnvalue_3 _heldby_2)
        (`Actor.K2_DestroyActor` HitObject)
        (`Actor.K2_DestroyActor` MainObject)
        (else
          ;[1 1 1] Player Not Holding Main Object Or Colliding Object
          (`GameplayStatics.SpawnEmitterAtLocation` "/Game/StarterContent/Particles/P_Explosion.P_Explosion" _impactpoint (struct) (5.0 5.0 5.0))
          (`Actor.K2_DestroyActor` HitObject)
          (`Actor.K2_DestroyActor` MainObject)
          (`|SpawnActorFromClass` ObjectClassToSpawn (`KismetMathLibrary.Conv_VectorToTransform` _impactpoint) "AlwaysSpawn" "OverrideRootScale" null null))))))