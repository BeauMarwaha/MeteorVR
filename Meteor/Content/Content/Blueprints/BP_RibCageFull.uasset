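; BP_RibCageFull is a pickup item, an intact rib cage that breaks a rib off into the hand when grabbed.
; On BeginPlay it sets its item icon.
; On Pickup it drops and destroys itself, spawns a broken rib cage and a single rib at its transform.
; It then sets the rib as the motion controller's attached actor and forwards the pickup to it.
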(event `self.ReceiveBeginPlay`
  ;[1 1 1] Set Item Icon
  (`AddComponent|NODE_AddBP_ItemIcon-0`))

(event `self.Pickup`
  (params (AttachTo :type "SceneComponent Object Reference"))
  (bind _returnvalue (`self.GetTransform`))
  ;[1 1 1] Pickup Actor should break off rib into hand and spawn broken ribs in its place
  (`self.Drop`)
  (`self.K2_DestroyActor`)
  (`|SpawnActorFromClass` "/Game/Content/Blueprints/BP_RibCageBroken.BP_RibCageBroken_C" _returnvalue "AlwaysSpawn" "OverrideRootScale" null null)
  (bind _returnvalue_2 (`|SpawnActorFromClass` "/Game/Content/Blueprints/BP_Rib.BP_Rib_C" _returnvalue "AlwaysSpawn" "OverrideRootScale" null null))
  (bind _asmotion_controller_component (cast `MotionControllerComponent` AttachTo))
  (bind _asbp_motion_controller (cast `/Game/VirtualRealityBP/Blueprints/BP_MotionController` (`ActorComponent.GetOwner` _asmotion_controller_component)))
  (set `/Game/VirtualRealityBP/Blueprints/BP_MotionController.AttachedActor` _returnvalue_2 _asbp_motion_controller)
  (`/Game/Content/Blueprints/BP_Rib.Pickup` _returnvalue_2 AttachTo))

(fn `UserConstructionScript`)